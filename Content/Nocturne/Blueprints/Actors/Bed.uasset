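; Bed prop actor for Nocturne, assembled from a set of instanced static mesh components.
; The construction script adds one instance to each numbered component, skipping number 8, at an identity transform.
; Each piece's placement therefore comes from its component rather than from the instance data.
; The event graph holds only disabled default events, so the bed has no gameplay logic here.
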(fn `UserConstructionScript`
  (`InstancedStaticMeshComponent.AddInstance` (`self.1`) (`KismetMathLibrary.MakeTransform` (0.0 0.0 0.0)))
  (`InstancedStaticMeshComponent.AddInstance` (`self.2`) (`KismetMathLibrary.MakeTransform` (0.0 0.0 0.0)))
  (`InstancedStaticMeshComponent.AddInstance` (`self.3`) (`KismetMathLibrary.MakeTransform` (0.0 0.0 0.0)))
  (`InstancedStaticMeshComponent.AddInstance` (`self.4`) (`KismetMathLibrary.MakeTransform` (0.0 0.0 0.0)))
  (`InstancedStaticMeshComponent.AddInstance` (`self.5`) (`KismetMathLibrary.MakeTransform` (0.0 0.0 0.0)))
  (`InstancedStaticMeshComponent.AddInstance` (`self.6`) (`KismetMathLibrary.MakeTransform` (0.0 0.0 0.0)))
  (`InstancedStaticMeshComponent.AddInstance` (`self.7`) (`KismetMathLibrary.MakeTransform` (0.0 0.0 0.0)))
  (`InstancedStaticMeshComponent.AddInstance` (`self.9`) (`KismetMathLibrary.MakeTransform` (0.0 0.0 0.0)))
  (`InstancedStaticMeshComponent.AddInstance` (`self.10`) (`KismetMathLibrary.MakeTransform` (0.0 0.0 0.0)))
  (`InstancedStaticMeshComponent.AddInstance` (`self.11`) (`KismetMathLibrary.MakeTransform` (0.0 0.0 0.0)))
  (`InstancedStaticMeshComponent.AddInstance` (`self.12`) (`KismetMathLibrary.MakeTransform` (0.0 0.0 0.0)))
  (`InstancedStaticMeshComponent.AddInstance` (`self.13`) (`KismetMathLibrary.MakeTransform` (0.0 0.0 0.0)))
  (`InstancedStaticMeshComponent.AddInstance` (`self.14`) (`KismetMathLibrary.MakeTransform` (0.0 0.0 0.0))))