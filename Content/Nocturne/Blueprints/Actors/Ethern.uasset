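; Ethern is a 2D flipbook character that walks along the X axis and deals heavy damage to the first player's pawn when its capsule hits it.
; Tick swaps idle and running flipbooks by speed, delaying the swap while airborne, and yaws the capsule to face the direction of travel.
; Move and SwitchMove events apply input along a direction flag and flip it, with no caller in this graph.
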(event `self.ReceiveBeginPlay`
  (`ActorComponent.SetIsReplicated` (`self.Sprite`) true))

(event `UpdateAnimation`
  ;[1 1 1] Handle Animation
  (`KismetSystemLibrary.Delay` (`KismetMathLibrary.SelectFloat` 0.0 0.6 (`NavMovementComponent.IsMovingOnGround` (`self.CharacterMovement`))))
  (`PaperFlipbookComponent.SetFlipbook` (`self.Sprite`) (select `bool` (> (`KismetMathLibrary.VSize` (`self.GetVelocity`)) 0.0) :`false` "/Game/2DSideScroller/Sprites/IdleAnimation.IdleAnimation" :`true` "/Game/2DSideScroller/Sprites/RunningAnimation.RunningAnimation" :!type "PaperFlipbook Object Reference")))

(event `self.ReceiveTick`
  (params (DeltaSeconds :type "Float (single-precision)"))
  ;[1 1 1] Tick - Updates animation
  (`self.UpdateAnimation`)
  (`/Engine/EditorBlueprintResources/StandardMacros.CompareFloat` (.x (`MovementComponent.Velocity` (`self.GetMovementComponent`)))
    (:`>`
      (`SceneComponent.K2_SetRelativeRotation` (`self.CapsuleComponent`) (`KismetMathLibrary.MakeRotator` 0.0 0.0 0.0) false false :!label _label))
    (:`==`
      (if (`self.bisMovingRight`)
        (goto _label)))
    (:`<`
      (`SceneComponent.K2_SetRelativeRotation` (`self.CapsuleComponent`) (`KismetMathLibrary.MakeRotator` 0.0 0.0 180.0) false false))))

(event `self.CapsuleComponent.OnComponentHit`
  (params (HitComponent :type "PrimitiveComponent Object Reference") (OtherActor :type "Actor Object Reference") (OtherComp :type "PrimitiveComponent Object Reference") (NormalImpulse :type "Vector Structure") (Hit :type "HitResult Structure (by ref)"))
  (bind _returnvalue (`GameplayStatics.GetPlayerPawn` 0))
  (if (== OtherActor _returnvalue)
    (`GameplayStatics.ApplyDamage` _returnvalue 100.0 null self)))

(event `Move`
  (`self.AddMovementInput` (1.0 0.0 0.0) (`KismetMathLibrary.SelectFloat` 1.0 -1.0 (`self.bisMovingRight`))))

(event `Switch Move`
  (set `self.bisMovingRight` (not (`self.bisMovingRight`))))

(fn `UserConstructionScript`)