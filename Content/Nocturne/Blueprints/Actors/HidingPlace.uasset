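; Hiding place pawn that the main character can occupy, with exit handled here.
; Its box overlap sets or clears itself as the character's HideObject and caches a reference to that character.
; Possession events track a Possessed flag.
; Interact input teleports the character's capsule back to its LastPosition, turns both point lights' intensity to zero and returns player control to the character.
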(event `self.ReceivePossessed`
  (params (NewController :type "Controller Object Reference"))
  (set `self.Possessed` true))

(event `self.ReceiveUnpossessed`
  (params (OldController :type "Controller Object Reference"))
  (set `self.Possessed` false))

(event `self.Box.OnComponentBeginOverlap`
  (params (OverlappedComponent :type "PrimitiveComponent Object Reference") (OtherActor :type "Actor Object Reference") (OtherComp :type "PrimitiveComponent Object Reference") (OtherBodyIndex :type Integer) (bFromSweep :type Boolean) (SweepResult :type "HitResult Structure (by ref)"))
  (bind _asmain_character (cast `/Game/Nocturne/Blueprints/Actors/MainCharacter` OtherActor))
  (set `/Game/Nocturne/Blueprints/Actors/MainCharacter.HideObject` self _asmain_character)
  (set `self.MainCharacter` _asmain_character))

(event `self.Box.OnComponentEndOverlap`
  (params (OverlappedComponent :type "PrimitiveComponent Object Reference") (OtherActor :type "Actor Object Reference") (OtherComp :type "PrimitiveComponent Object Reference") (OtherBodyIndex :type Integer))
  (bind _asmain_character (cast `/Game/Nocturne/Blueprints/Actors/MainCharacter` OtherActor))
  (set `/Game/Nocturne/Blueprints/Actors/MainCharacter.HideObject` null _asmain_character))

(event `InputAction|Interact`
  (params (Key :type "Key Structure" :default "AnyKey"))
  (bind _maincharacter (`self.MainCharacter`))
  (:`Pressed`
    (`/Engine/EditorBlueprintResources/StandardMacros.IsValid` _maincharacter
      (:`Is Valid`
        (`SceneComponent.K2_SetWorldLocation` (`Character.CapsuleComponent` _maincharacter) (`/Game/Nocturne/Blueprints/Actors/MainCharacter.LastPosition` _maincharacter) false true)
        (`LightComponent.SetIntensity` (`self.PointLight1`) 0.0)
        (`LightComponent.SetIntensity` (`self.PointLight`) 0.0)
        (`Controller.Possess` (`GameplayStatics.GetPlayerController` 0) _maincharacter)))))

(fn `UserConstructionScript`)