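; LockedDoor is a door actor, referenced by the player as the next-level door, that unlocks once the player has held all its required puzzle keys.
; Each tick it removes every key in the MainCharacter's PuzzleKey array from its own PuzzleKey array and sets IsUnlocked when that array is empty.
; Its Box overlap sets itself as the character's NextLevelDoor on entry and clears that reference on exit.
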(event `self.ReceiveTick`
  (params (DeltaSeconds :type "Float (single-precision)"))
  (bind _puzzlekey (`self.PuzzleKey`))
  (bind _asmain_character (cast `/Game/Nocturne/Blueprints/Actors/MainCharacter` (`GameplayStatics.GetPlayerCharacter` 0)))
  (for _array_element (`/Game/Nocturne/Blueprints/Actors/MainCharacter.PuzzleKey` _asmain_character)
    (`KismetArrayLibrary.Array_RemoveItem` _puzzlekey _array_element))
  (if (== 0 (`KismetArrayLibrary.Array_Length` _puzzlekey))
    (set `self.isUnlocked` true)))

(event `self.Box.OnComponentBeginOverlap`
  (params (OverlappedComponent :type "PrimitiveComponent Object Reference") (OtherActor :type "Actor Object Reference") (OtherComp :type "PrimitiveComponent Object Reference") (OtherBodyIndex :type Integer) (bFromSweep :type Boolean) (SweepResult :type "HitResult Structure (by ref)"))
  (bind _asmain_character (cast `/Game/Nocturne/Blueprints/Actors/MainCharacter` OtherActor))
  (set `/Game/Nocturne/Blueprints/Actors/MainCharacter.NextLevelDoor` self _asmain_character))

(event `self.Box.OnComponentEndOverlap`
  (params (OverlappedComponent :type "PrimitiveComponent Object Reference") (OtherActor :type "Actor Object Reference") (OtherComp :type "PrimitiveComponent Object Reference") (OtherBodyIndex :type Integer))
  (bind _asmain_character (cast `/Game/Nocturne/Blueprints/Actors/MainCharacter` OtherActor))
  (set `/Game/Nocturne/Blueprints/Actors/MainCharacter.NextLevelDoor` null _asmain_character))

(fn `UserConstructionScript`)