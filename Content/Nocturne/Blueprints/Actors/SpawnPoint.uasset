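; SpawnPoint is a proximity-triggered actor that spawns an Ethern when the MainCharacter comes close.
; Overlapping the outer trigger plays a clock sound cue.
; Overlapping the inner trigger spawns an Ethern with a default controller at the point, using the player's negated rotation, but only if none exists in the level.
; The spawn point then destroys itself, whether or not it spawned one.
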(event `self.Outer Trigger.OnComponentBeginOverlap`
  (params (OverlappedComponent :type "PrimitiveComponent Object Reference") (OtherActor :type "Actor Object Reference") (OtherComp :type "PrimitiveComponent Object Reference") (OtherBodyIndex :type Integer) (bFromSweep :type Boolean) (SweepResult :type "HitResult Structure (by ref)"))
  (cast `/Game/Nocturne/Blueprints/Actors/MainCharacter` OtherActor)
  (`AudioComponent.Play` (`self.clockCue`) 0.0))

(event `self.Inner Trigger.OnComponentBeginOverlap`
  (params (OverlappedComponent :type "PrimitiveComponent Object Reference") (OtherActor :type "Actor Object Reference") (OtherComp :type "PrimitiveComponent Object Reference") (OtherBodyIndex :type Integer) (bFromSweep :type Boolean) (SweepResult :type "HitResult Structure (by ref)"))
  (bind _asmain_character (cast `/Game/Nocturne/Blueprints/Actors/MainCharacter` OtherActor))
  (bind _outactors (`GameplayStatics.GetAllActorsOfClass` "/Game/Nocturne/Blueprints/Actors/Ethern.Ethern_C"))
  (if (== (`KismetArrayLibrary.Array_Length` _outactors) 0)
    (bind _returnvalue (`|SpawnActorFromClass` "/Game/Nocturne/Blueprints/Actors/Ethern.Ethern_C" (`KismetMathLibrary.MakeTransform` (`self.K2_GetActorLocation`) (`KismetMathLibrary.NegateRotator` (.rotation (`self.GetTransform` _asmain_character)))) "Undefined" "OverrideRootScale"))
    (`Pawn.SpawnDefaultController` _returnvalue))
  (`self.K2_DestroyActor`))

(fn `UserConstructionScript`)