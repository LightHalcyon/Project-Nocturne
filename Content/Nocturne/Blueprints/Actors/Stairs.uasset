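; Stairs actor that changes how the MainCharacter moves while inside its Box trigger.
; On begin overlap it switches the character's movement mode to Flying and nudges the capsule a fixed distance along world +Y.
; On end overlap it restores Walking and applies the opposite Y offset, using non-swept location sets on the capsule.
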(event `self.Box.OnComponentBeginOverlap`
  (params (OverlappedComponent :type "PrimitiveComponent Object Reference") (OtherActor :type "Actor Object Reference") (OtherComp :type "PrimitiveComponent Object Reference") (OtherBodyIndex :type Integer) (bFromSweep :type Boolean) (SweepResult :type "HitResult Structure (by ref)"))
  (bind _asmain_character (cast `/Game/Nocturne/Blueprints/Actors/MainCharacter` OtherActor))
  (`CharacterMovementComponent.SetMovementMode` (`Character.CharacterMovement` _asmain_character) "MOVE_Flying" 0)
  (bind _capsulecomponent (`Character.CapsuleComponent` _asmain_character))
  (`SceneComponent.K2_SetWorldLocation` _capsulecomponent (`KismetMathLibrary.MakeVector` (.x (`SceneComponent.K2_GetComponentLocation` _capsulecomponent)) (+ (.y (`SceneComponent.K2_GetComponentLocation` _capsulecomponent)) 13.0) (.z (`SceneComponent.K2_GetComponentLocation` _capsulecomponent))) false false))

(event `self.Box.OnComponentEndOverlap`
  (params (OverlappedComponent :type "PrimitiveComponent Object Reference") (OtherActor :type "Actor Object Reference") (OtherComp :type "PrimitiveComponent Object Reference") (OtherBodyIndex :type Integer))
  (bind _asmain_character (cast `/Game/Nocturne/Blueprints/Actors/MainCharacter` OtherActor))
  (`CharacterMovementComponent.SetMovementMode` (`Character.CharacterMovement` _asmain_character) "MOVE_Walking" 0)
  (bind _capsulecomponent (`Character.CapsuleComponent` _asmain_character))
  (`SceneComponent.K2_SetWorldLocation` _capsulecomponent (`KismetMathLibrary.MakeVector` (.x (`SceneComponent.K2_GetComponentLocation` _capsulecomponent)) (- (.y (`SceneComponent.K2_GetComponentLocation` _capsulecomponent)) 13.0) (.z (`SceneComponent.K2_GetComponentLocation` _capsulecomponent))) false false))

(fn `UserConstructionScript`)